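; Cock Blaster projectile weapon Blueprint that overrides FireProjectile to launch shots from its MordhauScene component instead of the supplied origin.
; Orientation, controller and expected delay pass unchanged to the parent implementation, which does the firing.
; Disconnected leftover nodes hold an authority-only chicken spawn with forward impulse and a multi-shot loop with random spread and recoil, none of which runs.
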(event EventFireProjectile
  (params (Origin :type Vector%20%28by%20ref%29 :default "0, 0, 0") (Orientation :type Rotator%20%28by%20ref%29 :default "0, 0, 0") (OwningController :type Controller%20Object%20Reference) (ExpectedDelay :type Float%20%28single-precision%29))
  (|CallParentFunction (Transformation|GetWorldLocation (Variables|Default|GetMordhauScene)) Orientation OwningController ExpectedDelay))

(fn ConstructionScript
  (|CallParentFunction))