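; Mordhau component that gives a controller's character three random weapons or equipment items each time it controls a new living character.
; A looping timer polls for a character change, then drops and destroys all gear except fists and spawns replacements with random customization, switching to the first.
; The item pool comes from the Mordhau singleton's equipment array and rebuilds when its length differs.
; An AddPerkToCharacter helper exists but is not called here.
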(event Custom|ServerSpawnGear
  (CallFunction|ValidateEquipment)
  (Utilities|FlowControl|Delay 0.2)
  (CallFunction|RandomGearSpawn))

(event Custom|CustomEvent_1)

(event Custom|CustomEvent_0
  (bind _returnvalue (CallFunction|SetCharacter))
  (if _returnvalue
    (CallFunction|ServerSpawnGear)))

(event EventBeginPlay
  (Utilities|FlowControl|Delay 0.35)
  (CallFunction|SetEquips)
  (bind _returnvalue (Utilities|Time|SetTimerbyEvent (delegate Custom|CustomEvent_0) 0.5 true))
  (Variables|Default|SetNewVar_0 _returnvalue))

(event EventEndPlay
  (params (EndPlayReason :type EEndPlayReason%20Enum :default "Destroyed"))
  (Utilities|Time|ClearandInvalidateTimerbyHandle (Variables|Default|GetNewVar_0))
  (|CallParentFunction EndPlayReason))

(fn AddPerktoCharacter
  (params (Perk :type Byte))
  (bind _character (Variables|Default|GetCharacter))
  (bind _returnvalue (Class|MordhauCharacter|GetCustomizationReplicationActor _character))
  (Utilities|IsValid _returnvalue
    (:Is%20Valid
      (if (Ability|HasAuthority _returnvalue)
        (if (Class|MordhauCharacter|HasPerk _character Perk)
          _
          (else
            (bind _returnvalue_2 (Game|ConstructObjectfromClass "/Script/Mordhau.CharacterProfileBPWrapper" self))
            (bind _output_get (Variables|/Script/Mordhau.CharacterProfileBPWrapper|SetProfile _returnvalue_2 (Variables|/Script/Mordhau.CustomizationReplicationActor|GetLastAssignedProfile _returnvalue)))
            (Class|CharacterProfileBPWrapper|TogglePerk _returnvalue_2 Perk)
            (Class|CustomizationReplicationActor|AssignDatafromProfile _returnvalue _output_get)
            (return)))))
    (:Is%20Not%20Valid
      _))
  (return))

(fn SetCharacter
  (bind _controller (Variables|Default|GetController))
  (bind _returnvalue (Class|MordhauPlayerController|GetControlledMordhauCharacter _controller true))
  (Development|PrintString "SetCharacter")
  (Utilities|IsValid _controller
    (:Is%20Valid
      (Utilities|IsValid _returnvalue
        (:Is%20Valid
          (if (Class|AdvancedCharacter|GetIsDead _returnvalue)
            (Variables|Default|SetCharacter 0 :!label _label)
            (elif (== (Variables|Default|GetCharacter) _returnvalue)
              _
              (else
                (Variables|Default|SetCharacter _returnvalue)
                (return true)))))
        (:Is%20Not%20Valid
          (goto _label))))
    (:Is%20Not%20Valid
      (goto _label)))
  (return false))

(fn OnRepPerk)

(fn RandomGearSpawn
  (bind _character (Variables|Default|GetCharacter))
  (for _array_element (Variables|/Script/Mordhau.MordhauCharacter|GetEquipment _character)
    (Utilities|IsValid _array_element
      (:Is%20Valid
        (Utilities|Casting|CastToBP_FistsWeapon _array_element
          (:CastFailed
            (bind _returnvalue (Class|MordhauCharacter|DropEquipment _character _array_element true))
            (Actor|DestroyActor _returnvalue))))))
  (for _index (range 0 2)
    (bind _returnvalue_2 (Game|SpawnActorfromClass (.OutItem (Utilities|Array|Random (Variables|Default|GetEquipment))) (Math|Conversions|ToTransform(Vector) (Transformation|GetActorLocation _character)) "Undefined" 0 _character))
    (bind _returnvalue_3 (Class|MordhauEquipment|GetRandomCustomization _returnvalue_2 false))
    (Class|MordhauEquipment|AssignCustomization _returnvalue_2 _returnvalue_3)
    (Class|MordhauCharacter|PickUp _character _returnvalue_2 -1)
    (if (== _index 0)
      (Class|MordhauCharacter|SwitchEquipment _character _returnvalue_2))))

(fn SetEquips
  (bind _output_get (LocalVariables|SetNewLocalVar_0 (Class|MordhauSingleton|GetEquipmentArray (Class|MordhauUtilityLibrary|GetMordhauSingleton))))
  (Utilities|Array|Clear (Variables|Default|GetEquipment))
  (for _array_element _output_get
    (Utilities|Array|Add (Variables|Default|GetEquipment) (Utilities|ResolveSoftReference _array_element)))
  (Variables|Default|SetEquipment (Variables|Default|GetEquipment)))

(fn ValidateEquipment
  (if (not (== (Utilities|Array|Length (Class|MordhauSingleton|GetEquipmentArray (Class|MordhauUtilityLibrary|GetMordhauSingleton))) (Utilities|Array|Length (Variables|Default|GetEquipment))))
    (CallFunction|SetEquips)))