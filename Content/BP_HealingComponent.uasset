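; Mordhau healing component that rewards a kill by giving health and stamina to the last damage source of the dead character.
; A looping one-second timer polls the Controller's pawn and binds the death handler whenever a new living character appears.
; On death, the handler casts that damage source to MordhauCharacter and applies replicated offsets.
; AddPerkToCharacter can add perks through the customization profile on authority, but nothing here calls it, despite the timer event's ServerSetPlayerPerk name.
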(event Custom|ServerSetPlayerPerk
  (bind _returnvalue (CallFunction|SetCharacter))
  (if _returnvalue
    (EventDispatchers|BindEventtoOnCharacterDied (Variables|Default|GetCharacter) (EventDispatchers|CreateEvent :!event Custom|OnCharacterDied))))

(event Custom|OnCharacterDied
  (params (Character :type Advanced%20Character%20Object%20Reference))
  (Development|PrintString "OnCharacterDied_HealingComponent")
  (bind _returnvalue (Class|AdvancedCharacter|GetLastNetDamageSource Character))
  (bind _asmordhau_character (Utilities|Casting|CastToMordhauCharacter _returnvalue))
  (Class|AdvancedCharacter|OffsetHealth _asmordhau_character 100 true)
  (Class|MordhauCharacter|OffsetStamina _asmordhau_character 100 true))

(event EventBeginPlay
  (Development|PrintString "BeginPlay_HealingComponent")
  (bind _returnvalue (Utilities|Time|SetTimerbyEvent (delegate Custom|ServerSetPlayerPerk) 1.0 true))
  (Variables|Default|SetNewVar_0 _returnvalue))

(event EventEndPlay
  (params (EndPlayReason :type EEndPlayReason%20Enum :default "Destroyed"))
  (Utilities|Time|ClearandInvalidateTimerbyHandle (Variables|Default|GetNewVar_0))
  (|CallParentFunction EndPlayReason))

(fn AddPerktoCharacter
  (params (Perk :type Byte))
  (bind _character (Variables|Default|GetCharacter))
  (bind _returnvalue (Class|MordhauCharacter|GetCustomizationReplicationActor _character))
  (Utilities|IsValid _returnvalue
    (:Is%20Valid
      (if (Ability|HasAuthority _returnvalue)
        (if (Class|MordhauCharacter|HasPerk _character Perk)
          _
          (else
            (bind _returnvalue_2 (Game|ConstructObjectfromClass "/Script/Mordhau.CharacterProfileBPWrapper" self))
            (bind _output_get (Variables|/Script/Mordhau.CharacterProfileBPWrapper|SetProfile _returnvalue_2 (Variables|/Script/Mordhau.CustomizationReplicationActor|GetLastAssignedProfile _returnvalue)))
            (Class|CharacterProfileBPWrapper|TogglePerk _returnvalue_2 Perk)
            (Class|CustomizationReplicationActor|AssignDatafromProfile _returnvalue _output_get)
            (return)))))
    (:Is%20Not%20Valid
      _))
  (return))

(fn SetCharacter
  (bind _controller (Variables|Default|GetController))
  (bind _returnvalue (Class|MordhauPlayerController|GetControlledMordhauCharacter _controller true))
  (Development|PrintString "SetCharacter_HealingComponent")
  (Utilities|IsValid _controller
    (:Is%20Valid
      (Utilities|IsValid _returnvalue
        (:Is%20Valid
          (if (Class|AdvancedCharacter|GetIsDead _returnvalue)
            (Variables|Default|SetCharacter 0 :!label _label)
            (elif (== (Variables|Default|GetCharacter) _returnvalue)
              _
              (else
                (Variables|Default|SetCharacter _returnvalue)
                (return true)))))
        (:Is%20Not%20Valid
          (goto _label))))
    (:Is%20Not%20Valid
      (goto _label)))
  (return false))

(fn OnRepPerk)