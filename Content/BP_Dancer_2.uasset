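; BP_Dancer_2 is a dancer character that plays a testing emote montage while its mesh continuously rotates.
; After short BeginPlay delays it assigns a profile and starts the emote, then sets a looping timer, apparently to replay it.
; Tick turns the mesh by a fixed step each frame, so spin speed depends on frame rate.
; GiveFists is empty, and the other animation debug nodes are disconnected.
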(event Custom|CustomEvent_0
  (Class|AdvancedCharacter|PlayAnim "/Game/Mordhau/Animations/RawClips/Misc/Emotes/Throatcut1/MTG_TestingEmote.MTG_TestingEmote" 1.0 true))

(event EventBeginPlay
  (Utilities|FlowControl|Delay 0.2)
  (Class|MordhauCharacter|AssignProfile (Variables|Default|GetNew%20Profile))
  (Utilities|FlowControl|Delay 0.5)
  (CallFunction|CustomEvent0)
  (Utilities|Time|SetTimerbyEvent (EventDispatchers|CreateEvent :!event Custom|CustomEvent_0) 11.15 true))

(event EventTick
  (params (DeltaSeconds :type Float%20%28single-precision%29))
  (bind _mesh (Variables|Character|GetMesh))
  (|CallParentFunction DeltaSeconds)
  (Transformation|SetRelativeRotation _mesh (Math|Rotator|Delta(Rotator) (Variables|/Script/Engine.SceneComponent|GetRelativeRotation _mesh) "0,1.000000, 0") false false))

(event EventOnPostProfileAssigned
  (|CallParentFunction))

(fn ConstructionScript
  (|CallParentFunction))

(fn GiveFists)