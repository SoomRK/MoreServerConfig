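; BP_Dancer_3 is a character that equips a randomly customized lute and emotes with it while its mesh spins.
; On BeginPlay, after short delays, it assigns a profile, spawns and equips the lute, then starts a looping timer, apparently to replay the lute emote montage.
; Tick nudges the mesh's relative rotation by a fixed step each frame, independent of delta time.
; Dance animation, kick and lute tone logic are left unconnected.
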(event Custom|CustomEvent_0
  (Class|AdvancedCharacter|PlayAnim "/Game/Mordhau/Animations/RawClips/Misc/Emotes/MTG_EmoteLute.MTG_EmoteLute" 1.0 false))

(event EventBeginPlay
  (Utilities|FlowControl|Delay 0.2)
  (Class|MordhauCharacter|AssignProfile (Variables|Default|GetNew%20Profile))
  (bind _returnvalue (Game|SpawnActorfromClass "/Game/Mordhau/Blueprints/Equipment/Weapons/Specific/Instruments/BP_Lute.BP_Lute_C" (Transformation|GetActorTransform) "Undefined" 0 0))
  (bind _returnvalue_2 (Class|MordhauEquipment|GetRandomCustomization _returnvalue false))
  (Class|MordhauEquipment|AssignCustomization _returnvalue _returnvalue_2)
  (Class|MordhauCharacter|PickUp _returnvalue -1)
  (Class|MordhauCharacter|SwitchEquipment _returnvalue)
  (Variables|Default|SetNewVar_0 _returnvalue)
  (Utilities|FlowControl|Delay 0.5)
  (CallFunction|CustomEvent0)
  (Utilities|Time|SetTimerbyEvent (EventDispatchers|CreateEvent :!event Custom|CustomEvent_0) 3.0 true))

(event EventTick
  (params (DeltaSeconds :type Float%20%28single-precision%29))
  (bind _mesh (Variables|Character|GetMesh))
  (|CallParentFunction DeltaSeconds)
  (Transformation|SetRelativeRotation _mesh (Math|Rotator|Delta(Rotator) (Variables|/Script/Engine.SceneComponent|GetRelativeRotation _mesh) "0,1.000000, 0") false false))

(event EventOnPostProfileAssigned
  (|CallParentFunction))

(fn ConstructionScript
  (|CallParentFunction))

(fn GiveFists)