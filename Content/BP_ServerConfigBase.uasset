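; Mordhau server-config actor that applies custom-config rules: gear restrictions, inventory slots, map equipment clearing, team colors, AFK-kick removal, MOTD.
; BeginPlay reads the config section, destroys itself on disabled maps, otherwise edits game mode/state and adds controller components after login.
; RepNotify variables apply bans, colors, AFK and MOTD settings, the latter two via local-controller components.
; Hardcoded PlayFab IDs unlock a chat-triggered gun with damage reduction, debug output and a special component.
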(event Custom|CustomEvent_4
  (params (NewPlayer :type Player%20Controller%20Object%20Reference))
  (bind _asbp_mordhau_player_controller (Utilities|Casting|CastToBP_MordhauPlayerController NewPlayer))
  (bind _returnvalue (AddComponent|AddBPSlotComponent _asbp_mordhau_player_controller (Math|Integer|Clamp(Integer) (Variables|Default|GetSlots) 1 9)))
  (Variables|/MoreServerConfig/BP_SlotComponent.BP_SlotComponent_C|SetController _returnvalue _asbp_mordhau_player_controller))

(event Custom|CustomEvent_1
  (params (Sender :type Actor%20Object%20Reference) (Msg :type String) (Type :type Name))
  (bind _asbp_mordhau_player_controller (Utilities|Casting|CastToBP_MordhauPlayerController Sender))
  (if (Utilities|Enum|Equal(Enum) (Class|MordhauPlayerController|GetPlayFabID _asbp_mordhau_player_controller) "A4C9257F2F946385")
    (if (.ReturnValue (CallFunction|MessageHasCommand Msg "SoomRK Mode Activate!"))
      (Utilities|IsValid (Class|MordhauPlayerController|GetControlledMordhauCharacter _asbp_mordhau_player_controller true) :!label _label
        (:Is%20Valid
          (if (Class|AdvancedCharacter|GetIsDead (Class|MordhauPlayerController|GetControlledMordhauCharacter _asbp_mordhau_player_controller true))
            (Utilities|FlowControl|Delay 1.0 :!label _label_2)
            (goto _label)
            (else
              (for _array_element (Variables|/Script/Mordhau.MordhauCharacter|GetEquipment (Class|MordhauPlayerController|GetControlledMordhauCharacter _asbp_mordhau_player_controller true))
                (Utilities|Casting|CastToBP_FistsWeapon _array_element
                  (:CastFailed
                    (Utilities|Casting|CastToBP_KickWeapon _array_element
                      (:CastFailed
                        (bind _returnvalue (Class|MordhauCharacter|DropEquipment (Class|MordhauPlayerController|GetControlledMordhauCharacter _asbp_mordhau_player_controller true) _array_element true))
                        (Actor|DestroyActor _returnvalue))))))
              (bind _returnvalue_2 (Game|SpawnActorfromClass "/MoreServerConfig/BP_SoomsGun.BP_SoomsGun_C" (Math|Conversions|ToTransform(Vector) (Transformation|GetActorLocation (Class|MordhauPlayerController|GetControlledMordhauCharacter _asbp_mordhau_player_controller true))) "Undefined" 0 (Class|MordhauPlayerController|GetControlledMordhauCharacter _asbp_mordhau_player_controller true)))
              (Class|MordhauCharacter|PickUp (Class|MordhauPlayerController|GetControlledMordhauCharacter _asbp_mordhau_player_controller true) _returnvalue_2 -1)
              (Class|MordhauCharacter|SwitchEquipment (Class|MordhauPlayerController|GetControlledMordhauCharacter _asbp_mordhau_player_controller true) _returnvalue_2)
              (Variables|/Script/Mordhau.AdvancedCharacter|SetReceivedDamageModifier (Class|MordhauPlayerController|GetControlledMordhauCharacter _asbp_mordhau_player_controller true) 0.05))))
        (:Is%20Not%20Valid
          (goto _label_2)))
      (elif (.ReturnValue (CallFunction|MessageHasCommand Msg ".SoomDebug"))
        (Utilities|FlowControl|Delay 0.2)
        (Default|RequestChatMessage _asbp_mordhau_player_controller (Utilities|String|Append "Max AFK Time == " (Utilities|String|ToString(Float) (Variables|/Script/Mordhau.MordhauPlayerController|GetMaxAFKTime _asbp_mordhau_player_controller))) false)
        (Default|RequestChatMessage _asbp_mordhau_player_controller (Utilities|String|Append "Max Message Length == " (Utilities|String|ToString(Integer) (Variables|/Game/Mordhau/Blueprints/BP_MordhauPlayerController.BP_MordhauPlayerController_C|GetMaxMessageLength _asbp_mordhau_player_controller))) false)))))

(event Custom|SetMOTD
  (Utilities|FlowControl|Delay 0.5)
  (bind _output_get (CallFunction|GetLocalController))
  (Utilities|IsValid _output_get
    (:Is%20Valid
      (AddComponent|AddBPMOTDComponent _output_get (Variables|Default|GetRuleInfos) (Variables|Default|GetDiscordURL) (Variables|Default|GetDiscordInfo) (Variables|Default|GetDonateInfo) (Variables|Default|GetDonateURL) (Variables|Default|GetTexture) (Variables|Default|GetImageURL) (Variables|Default|GetBannerURL) (Variables|Default|GetX) (Variables|Default|GetY)))))

(event Custom|SetAFK
  (Utilities|FlowControl|Delay 1.0)
  (bind _output_get (CallFunction|GetLocalController))
  (if (Variables|Default|GetAFKDisabled)
    (Utilities|IsValid _output_get
      (:Is%20Valid
        (AddComponent|AddBPAFKRemovalComponent _output_get)))
    (elif (Variables|Default|GetAFKDisabledAdmin)
      (if (Class|MordhauPlayerController|IsAdmin _output_get)
        (AddComponent|AddBPAFKRemovalComponent _output_get)))))

(event Custom|CustomEvent_0
  (params (NewPlayer :type Player%20Controller%20Object%20Reference))
  (bind _asbp_mordhau_player_controller (Utilities|Casting|CastToBP_MordhauPlayerController NewPlayer))
  (bind _returnvalue (AddComponent|AddBPMasterComponent _asbp_mordhau_player_controller 3))
  (Variables|/MoreServerConfig/BP_MasterComponent.BP_MasterComponent_C|SetController _returnvalue _asbp_mordhau_player_controller))

(event Custom|CustomEvent_5
  (params (NewPlayer :type Player%20Controller%20Object%20Reference))
  (bind _asbp_mordhau_player_controller (Utilities|Casting|CastToBP_MordhauPlayerController NewPlayer))
  (if (Utilities|Enum|Equal(Enum) (Class|MordhauPlayerController|GetPlayFabID _asbp_mordhau_player_controller) "56DD685D95FCA828")
    (bind _returnvalue (AddComponent|AddBPDutchComponent _asbp_mordhau_player_controller))
    (Variables|/MoreServerConfig/BP_DutchComponent.BP_DutchComponent_C|SetController _returnvalue _asbp_mordhau_player_controller)))

(event Custom|CustomEvent
  (params (NewPlayer :type Player%20Controller%20Object%20Reference))
  (bind _asbp_mordhau_player_controller (Utilities|Casting|CastToBP_MordhauPlayerController NewPlayer))
  (bind _returnvalue (AddComponent|AddBPMasterComponent _asbp_mordhau_player_controller 11))
  (Variables|/MoreServerConfig/BP_MasterComponent.BP_MasterComponent_C|SetController _returnvalue _asbp_mordhau_player_controller))

(event Custom|ChangeColors
  (bind _team0array (Variables|Default|GetTeam0Array))
  (bind _secondaryarray (Variables|Default|GetSecondaryArray))
  (Utilities|FlowControl|Delay 1.0)
  (bind _asbp_mordhau_game_state (Utilities|Casting|CastToBP_MordhauGameState (Game|GetGameState)))
  (Utilities|FlowControl|Sequence
    (:then_0
      (if (> (Utilities|Array|Length _team0array) 0)
        (Variables|/Script/Mordhau.MordhauGameState|SetTeamColors _asbp_mordhau_game_state _team0array)))
    (:then_1
      (if (> (Utilities|Array|Length _secondaryarray) 0)
        (Variables|/Script/Mordhau.MordhauGameState|SetSecondaryTeamColors _asbp_mordhau_game_state _secondaryarray)))))

(event Custom|CustomEvent_6
  (CallFunction|ChangeColors))

(event EventBeginPlay
  (Development|PrintString "ServerConfig_BeginPlay" true true "(R=1.000000,G=0.019382,B=0.000000,A=1.000000)" 5.0)
  (bind _returnvalue (CallFunction|GetConfig))
  (if _returnvalue
    (Actor|DestroyActor)
    (else
      (|CallParentFunction)
      (Utilities|FlowControl|Delay 1.0)
      (Utilities|FlowControl|Sequence
        (:then_0
          (if (Variables|Default|GetPeasantOnly)
            (Variables|Default|SetBannedEquip_Peasant (Variables|Default|GetBannedEquip_Peasant))
            (bind _asbp_mordhau_game_mode (Utilities|Casting|CastToBP_MordhauGameMode (Game|GetGameMode)))
            (EventDispatchers|BindEventtoOnAfterLogin _asbp_mordhau_game_mode (delegate Custom|CustomEvent_0))
            (Utilities|FlowControl|Delay 1.0)
            (CallFunction|ClearNobleGearPeasant)))
        (:then_1
          (if (Variables|Default|GetDwarfOnly)
            (bind _asbp_mordhau_game_mode_2 (Utilities|Casting|CastToBP_MordhauGameMode (Game|GetGameMode)))
            (EventDispatchers|BindEventtoOnAfterLogin _asbp_mordhau_game_mode_2 (delegate Custom|CustomEvent))))
        (:then_2
          (if (not (== (Variables|Default|GetSlots) -1))
            (bind _asbp_mordhau_game_mode_3 (Utilities|Casting|CastToBP_MordhauGameMode (Game|GetGameMode)))
            (EventDispatchers|BindEventtoOnAfterLogin _asbp_mordhau_game_mode_3 (delegate Custom|CustomEvent_4))))
        (:then_3
          (if (Variables|Default|GetClearMapEquipment)
            (CallFunction|ClearRandomEquipment)))
        (:then_4
          (if (Variables|Default|GetFistsOnly)
            (Variables|Default|SetBannedEquip_Fists (Variables|Default|GetBannedEquip_Fists))
            (Utilities|FlowControl|Delay 1.0)
            (CallFunction|ClearNobleGearFists)))
        (:then_5
          (bind _asbp_mordhau_game_mode_4 (Utilities|Casting|CastToBP_MordhauGameMode (Game|GetGameMode)))
          (EventDispatchers|BindEventtoOnMessageBroadcasted _asbp_mordhau_game_mode_4 (delegate Custom|CustomEvent_1))
          (EventDispatchers|BindEventtoOnAfterLogin _asbp_mordhau_game_mode_4 (delegate Custom|CustomEvent_5)))))))

(fn ConstructionScript
  (|CallParentFunction))

(fn GetConfig
  (bind _section_name (Variables|Default|GetSection%20Name))
  (bind _section_name_2 (Variables|Default|GetSection%20Name))
  (bind (_isvalid _returnvalue) (Class|MordhauUtilityLibrary|GetCustomConfigVarInt _section_name "InventorySlots"))
  (bind (_isvalid_2 _returnvalue_2) (Class|MordhauUtilityLibrary|GetCustomConfigVarBool _section_name "DwarfOnly"))
  (bind (_isvalid_3 _returnvalue_3) (Class|MordhauUtilityLibrary|GetCustomConfigVarBool _section_name "DisableAfkKickAdmin"))
  (bind (_isvalid_4 _returnvalue_4) (Class|MordhauUtilityLibrary|GetCustomConfigVarBool _section_name "DisableAfkKick"))
  (bind (_isvalid_5 _returnvalue_5) (Class|MordhauUtilityLibrary|GetCustomConfigVarColor _section_name_2 "Team1SecondaryColor"))
  (bind (_isvalid_6 _returnvalue_6) (Class|MordhauUtilityLibrary|GetCustomConfigVarColor _section_name_2 "Team0SecondaryColor"))
  (bind (_isvalid_7 _returnvalue_7) (Class|MordhauUtilityLibrary|GetCustomConfigVarColor _section_name_2 "Team0PrimaryColor"))
  (bind (_isvalid_8 _returnvalue_8) (Class|MordhauUtilityLibrary|GetCustomConfigVarColor _section_name_2 "Team1PrimaryColor"))
  (bind (_isvalid_9 _returnvalue_9) (Class|MordhauUtilityLibrary|GetCustomConfigVarBool _section_name "PeasantOnly"))
  (bind (_isvalid_10 _returnvalue_10) (Class|MordhauUtilityLibrary|GetCustomConfigVarBool _section_name "EnableMOTD"))
  (bind (_isvalid_11 _returnvalue_11) (Class|MordhauUtilityLibrary|GetCustomConfigVarBool _section_name "ClearMapEquipment"))
  (bind (_isvalid_12 _returnvalue_12) (Class|MordhauUtilityLibrary|GetCustomConfigVarBool _section_name "DisableSpamFilter"))
  (bind (_isvalid_13 _returnvalue_13) (Class|MordhauUtilityLibrary|GetCustomConfigVarString _section_name "BannerURL"))
  (bind (_isvalid_14 _returnvalue_14) (Class|MordhauUtilityLibrary|GetCustomConfigVarString _section_name "DonateURL"))
  (bind (_arraysize _returnvalue_15) (Class|MordhauUtilityLibrary|GetCustomConfigVarArray _section_name "RuleInfo"))
  (bind (_isvalid_15 _returnvalue_16) (Class|MordhauUtilityLibrary|GetCustomConfigVarString _section_name "DiscordURL"))
  (bind (_isvalid_16 _returnvalue_17) (Class|MordhauUtilityLibrary|GetCustomConfigVarString _section_name "DiscordInfo"))
  (bind (_isvalid_17 _returnvalue_18) (Class|MordhauUtilityLibrary|GetCustomConfigVarString _section_name "DonateInfo"))
  (bind (_isvalid_18 _returnvalue_19) (Class|MordhauUtilityLibrary|GetCustomConfigVarString _section_name "ImageURL"))
  (bind (_isvalid_19 _returnvalue_20) (Class|MordhauUtilityLibrary|GetCustomConfigVarFloat _section_name "MOTDHeight"))
  (bind (_arraysize_2 _returnvalue_21) (Class|MordhauUtilityLibrary|GetCustomConfigVarArray _section_name "DisableOnMap"))
  (bind (_isvalid_20 _returnvalue_22) (Class|MordhauUtilityLibrary|GetCustomConfigVarFloat _section_name "MOTDWidth"))
  (bind (_isvalid_21 _returnvalue_23) (Class|MordhauUtilityLibrary|GetCustomConfigVarBool _section_name "DisableSpamFilterAdmin"))
  (bind (_isvalid_22 _returnvalue_24) (Class|MordhauUtilityLibrary|GetCustomConfigVarBool _section_name "FistsOnly"))
  (bind (_isvalid_23 _returnvalue_25) (Class|MordhauUtilityLibrary|GetCustomConfigVarBool _section_name "UseCustomTeamColors"))
  (Utilities|FlowControl|Sequence
    (:then_0
      (if (> _arraysize_2 0)
        (bind _returnvalue_26 (Game|GetCurrentLevelName false))
        (LocalVariables|SetTemp _returnvalue_26)
        (for _array_element _returnvalue_21
          (if (Utilities|Enum|Equal(Enum) _array_element (LocalVariables|GetTemp))
            (return true)))))
    (:then_1
      (if (and _isvalid_9 _returnvalue_9)
        (Variables|Default|SetPeasantOnly true)
        (else
          (Variables|Default|SetPeasantOnly false))))
    (:then_2
      (if (and _isvalid_22 _returnvalue_24)
        (Variables|Default|SetFistsOnly true)
        (else
          (Variables|Default|SetFistsOnly false))))
    (:then_3
      (if (and _isvalid_4 _returnvalue_4)
        (Variables|Default|SetDisableAFK true)
        (else
          (Variables|Default|SetDisableAFK false))))
    (:then_4
      (if (and _isvalid_3 _returnvalue_3)
        (Variables|Default|SetDisableAFK_Admin true)
        (else
          (Variables|Default|SetDisableAFK_Admin false))))
    (:then_5
      (if (and _isvalid_2 _returnvalue_2)
        (Variables|Default|SetDwarfOnly true)
        (else
          (Variables|Default|SetDwarfOnly false))))
    (:then_6
      (if _isvalid
        (Variables|Default|SetSlots _returnvalue)
        (else
          (Variables|Default|SetSlots -1))))
    (:then_7
      (if (and _isvalid_11 _returnvalue_11)
        (Variables|Default|SetClearMapEquipment true)
        (else
          (Variables|Default|SetClearMapEquipment false))))
    (:then_8
      (if (and _isvalid_23 _returnvalue_25)
        (Variables|Default|SetUseCustomTeamColors true)
        (Utilities|FlowControl|Sequence
          (:then_0
            (if (and _isvalid_7 _isvalid_6)
              (Variables|Default|SetTeam0Array (Utilities|Array|MakeArray _returnvalue_7 _returnvalue_6))))
          (:then_1
            (if (and _isvalid_8 _isvalid_5)
              (Variables|Default|SetSecondaryArray (Utilities|Array|MakeArray _returnvalue_8 _returnvalue_5)))))
        (else
          (Variables|Default|SetUseCustomTeamColors false))))
    (:then_9
      (if (and _isvalid_12 _returnvalue_12)
        (Variables|Default|SetDisableSpamFilter true)
        (else
          (Variables|Default|SetDisableSpamFilter false))))
    (:then_10
      (if (and _isvalid_21 _returnvalue_23)
        (Variables|Default|SetDisableSpamFilter_Admin true)
        (else
          (Variables|Default|SetDisableSpamFilter_Admin false))))
    (:then_11
      (Utilities|FlowControl|Sequence
        (:then_0
          (if _isvalid_15
            (Variables|Default|SetDiscordURL _returnvalue_16)))
        (:then_1
          (if _isvalid_16
            (Variables|Default|SetDiscordInfo _returnvalue_17)))
        (:then_2
          (if (> _arraysize 0)
            (for (_array_element_2 _array_index) _returnvalue_15
              (Utilities|Array|AddUnique (Variables|Default|GetRuleInfos) (Utilities|String|Append (Utilities|String|ToString(Integer) (+ _array_index 1)) ".)" " " _array_element_2)))
            (Variables|Default|SetRuleInfos (Variables|Default|GetRuleInfos))))
        (:then_3
          (if _isvalid_14
            (Variables|Default|SetDonateURL _returnvalue_14)))
        (:then_4
          (if _isvalid_17
            (Variables|Default|SetDonateInfo _returnvalue_18)))
        (:then_5
          (if _isvalid_18
            (Variables|Default|SetImageURL _returnvalue_19)))
        (:then_6
          (if _isvalid_13
            (Variables|Default|SetBannerURL _returnvalue_13)))
        (:then_7
          (if (and _isvalid_20 _isvalid_19)
            (Variables|Default|SetX (Math|Float|Clamp(Float) _returnvalue_22 0.0 8.7e+02))
            (Variables|Default|SetY (Math|Float|Clamp(Float) _returnvalue_20 0.0 2.2e+02))
            (else
              (Variables|Default|SetX 8.7e+02)
              (Variables|Default|SetY 2.2e+02))))
        (:then_8
          (if (and _isvalid_10 _returnvalue_10)
            (Variables|Default|SetEnableMOTD true)
            (else
              (Variables|Default|SetEnableMOTD false))))))
    (:then_12
      (return false))))

(fn MessageHasCommand
  (params (Message :type String) (Command :type String))
  (LocalVariables|SetMessageX Message)
  (LocalVariables|SetCommandX Command)
  (if (Utilities|String|StartsWith (LocalVariables|GetMessageX) (LocalVariables|GetCommandX))
    (return true (Utilities|String|GetSubstring (LocalVariables|GetMessageX) (Utilities|String|Len (LocalVariables|GetCommandX)) (- (Utilities|String|Len (LocalVariables|GetMessageX)) (Utilities|String|Len (LocalVariables|GetCommandX)))))
    (else
      (return false ""))))

(fn ParseMessage
  (params (Message :type String))
  (bind _output_get (LocalVariables|SetTemp Message))
  (if (Utilities|String|Contains _output_get " ")
    (if (Utilities|Enum|Equal(Enum) (.RightS (Utilities|String|Split _output_get " ")) "")
      _
      (else
        (bind (_array_element _returnvalue) (CallFunction|GetPlayer (.LeftS (Utilities|String|Split _output_get " "))))
        (if _returnvalue
          (return (.LeftS (Utilities|String|Split _output_get " ")) (Math|Conversions|ToInteger(Byte) (.RightS (Utilities|String|Split _output_get " "))) _array_element)
          (else
            (return "invalid" 0 0))))))
  (return "invalid" (Math|Conversions|ToInteger(Byte) _output_get) 0))

(fn GetPlayer
  (params (Player :type String))
  (bind _asbp_mordhau_game_state (Utilities|Casting|CastToBP_MordhauGameState (Game|GetGameState)))
  (for _array_element (Variables|/Script/Engine.GameStateBase|GetPlayerArray _asbp_mordhau_game_state)
    (if (Utilities|String|Contains (PlayerState|GetPlayerName _array_element) Player)
      (return _array_element true)))
  (return 0 false))

(fn OnRepPeasantOnly)

(fn OnRepFistsOnly)

(fn OnRepDisableAFKAdmin
  (if (Variables|Default|GetDisableAFK_Admin)
    (Variables|Default|SetAFKDisabledAdmin true)
    (CallFunction|SetAFK)))

(fn OnRepDisableAFK
  (if (Variables|Default|GetDisableAFK)
    (Variables|Default|SetAFKDisabled true)
    (CallFunction|SetAFK)))

(fn OnRepBannedEquipFists
  (bind _bannedequip_fists (Variables|Default|GetBannedEquip_Fists))
  (if (Variables|Default|GetFistsOnly)
    (bind _asbp_mordhau_game_state (Utilities|Casting|CastToBP_MordhauGameState (Game|GetGameState)))
    (bind _output_get (LocalVariables|SetTemp (Class|MordhauSingleton|GetEquipmentArray (Class|MordhauUtilityLibrary|GetMordhauSingleton))))
    (for _array_element _output_get
      (Utilities|Array|AddUnique _bannedequip_fists (Utilities|ResolveSoftReference _array_element)))
    (Utilities|Set|AddItems (Variables|/Script/Mordhau.MordhauGameState|GetBannedEquipment _asbp_mordhau_game_state) _bannedequip_fists)
    (Variables|/Script/Mordhau.MordhauGameState|SetBannedEquipment _asbp_mordhau_game_state (Variables|/Script/Mordhau.MordhauGameState|GetBannedEquipment _asbp_mordhau_game_state))))

(fn OnRepDwarfOnly)

(fn ClearRandomEquipment
  (Utilities|FlowControl|Sequence
    (:then_0
      (bind _asbp_mordhau_game_mode (Utilities|Casting|CastToBP_MordhauGameMode (Game|GetGameMode)))
      (Variables|/Game/Mordhau/Blueprints/GameModes/BP_MordhauGameMode.BP_MordhauGameMode_C|SetNoEquipmentSpawners _asbp_mordhau_game_mode true)
      (bind _asbp_mordhau_game_state (Utilities|Casting|CastToBP_MordhauGameState (Game|GetGameState)))
      (Variables|/Game/Mordhau/Blueprints/GameModes/BP_MordhauGameState.BP_MordhauGameState_C|SetNoPreplacedEquipment _asbp_mordhau_game_state true))
    (:then_1
      (bind _outactors (Actor|GetAllActorsOfClass "/Game/Mordhau/Blueprints/BP_ActorSpawnController.BP_ActorSpawnController_C"))
      (if (> (Utilities|Array|Length _outactors) 0)
        (for _array_element _outactors
          (Utilities|Array|Clear (Variables|/Game/Mordhau/Blueprints/BP_ActorSpawnController.BP_ActorSpawnController_C|GetEquipment _array_element))))
      (bind _outactors_2 (Actor|GetAllActorsOfClass "/Game/Mordhau/Blueprints/Equipment/BP_RandomEquipment.BP_RandomEquipment_C"))
      (if (> (Utilities|Array|Length _outactors_2) 0)
        (for _array_element_2 _outactors_2
          (Networking|SetReplicates _array_element_2 true)
          (Actor|DestroyActor _array_element_2))))))

(fn ClearNobleGearPeasant
  (bind _outactors (Actor|GetAllActorsOfClass "/Game/Mordhau/Blueprints/GameModes/Battle/BP_FrontlineKillObjective.BP_FrontlineKillObjective_C"))
  (if (> (Utilities|Array|Length _outactors) 0)
    (for _array_element _outactors
      (Utilities|FlowControl|Sequence
        (:then_0
          (bind _returnvalue (Class|MordhauCharacter|GetCustomizationReplicationActor _array_element))
          (Class|CustomizationReplicationActor|AssignDatafromProfile _returnvalue (.OutItem (Utilities|Array|Random (Variables|Default|GetPeasantProfiles))))
          (Class|MordhauCharacter|SetCustomizationReplicationActor _array_element _returnvalue)
          (Class|MordhauCharacter|OnPostProfileAssigned _array_element))
        (:then_1
          (for _array_element_2 (Variables|/Script/Mordhau.MordhauCharacter|GetEquipment _array_element)
            (Utilities|Casting|CastToBP_KickWeapon _array_element_2
              (:CastFailed
                (bind _returnvalue_2 (Class|MordhauCharacter|DropEquipment _array_element _array_element_2 true))
                (Actor|DestroyActor _returnvalue_2))))
          (bind _returnvalue_3 (Game|SpawnActorfromClass "/MoreServerConfig/BP_MetalShovel_Noble.BP_MetalShovel_Noble_C" (Transformation|GetActorTransform _array_element) "Undefined" 0 _array_element))
          (Class|MordhauCharacter|PickUp _array_element _returnvalue_3 -1)
          (Class|MordhauCharacter|SwitchEquipment _array_element _returnvalue_3))))))

(fn ClearNobleGearFists
  (bind _outactors (Actor|GetAllActorsOfClass "/Game/Mordhau/Blueprints/GameModes/Battle/BP_FrontlineKillObjective.BP_FrontlineKillObjective_C"))
  (if (> (Utilities|Array|Length _outactors) 0)
    (for _array_element _outactors
      (for _array_element_2 (Variables|/Script/Mordhau.MordhauCharacter|GetEquipment _array_element)
        (Utilities|Casting|CastToBP_KickWeapon _array_element_2
          (:CastFailed
            (bind _returnvalue (Class|MordhauCharacter|DropEquipment _array_element _array_element_2 true))
            (Actor|DestroyActor _returnvalue))))
      (bind _returnvalue_2 (Game|SpawnActorfromClass "/Game/Mordhau/Blueprints/Equipment/Weapons/BP_PugilistFistsWeapon.BP_PugilistFistsWeapon_C" (Transformation|GetActorTransform _array_element) "Undefined" 0 _array_element))
      (Class|MordhauCharacter|PickUp _array_element _returnvalue_2 -1)
      (Class|MordhauCharacter|SwitchEquipment _array_element _returnvalue_2))))

(fn OnRepClearMapEquipment
  (if (Variables|Default|GetClearMapEquipment)
    (CallFunction|ClearRandomEquipment)))

(fn OnRepSectionName)

(fn OnRepSlots)

(fn Debug
  (bind _asbp_skirmish_game_state (Utilities|Casting|CastToBP_SkirmishGameState (Game|GetGameState)))
  (for (_array_element _array_index) (Variables|/Script/Mordhau.MordhauGameState|GetTeamColors _asbp_skirmish_game_state)
    (Class|MordhauUtilityLibrary|SetCustomConfigVarColor "ServerConfigBase" (Utilities|String|Append "Primary" (Utilities|String|ToString(Integer) _array_index)) _array_element))
  (for (_array_element_2 _array_index_2) (Variables|/Script/Mordhau.MordhauGameState|GetSecondaryTeamColors _asbp_skirmish_game_state)
    (Class|MordhauUtilityLibrary|SetCustomConfigVarColor "ServerConfigBase" (Utilities|String|Append "Secondary" (Utilities|String|ToString(Integer) _array_index_2)) _array_element_2)))

(fn OnRepUseCustomTeamColors
  (if (Variables|Default|GetUseCustomTeamColors)
    (CallFunction|ChangeColors)))

(fn SetupColors)

(fn NewFunction0)

(fn OnRepBannedEquipPeasant
  (if (Variables|Default|GetPeasantOnly)
    (bind _asbp_mordhau_game_state (Utilities|Casting|CastToBP_MordhauGameState (Game|GetGameState)))
    (Utilities|Set|AddItems (Variables|/Script/Mordhau.MordhauGameState|GetBannedEquipment _asbp_mordhau_game_state) (Variables|Default|GetBannedEquip_Peasant))
    (Variables|/Script/Mordhau.MordhauGameState|SetBannedEquipment _asbp_mordhau_game_state (Variables|/Script/Mordhau.MordhauGameState|GetBannedEquipment _asbp_mordhau_game_state))))

(fn OnRepTeam0Array)

(fn OnRepSecondaryArray)

(fn OnRepDisableSpamFilter)

(fn OnRepDisableSpamFilterAdmin)

(fn GetLocalController
  (bind _returnvalue (Game|GetPlayerController 0))
  (if (Pawn|IsLocalPlayerController _returnvalue)
    (bind _asbp_mordhau_player_controller (Utilities|Casting|CastToBP_MordhauPlayerController _returnvalue)
      (:then
        (bind _output_get (LocalVariables|SetTemp _asbp_mordhau_player_controller))
        (return _output_get))
      (:CastFailed
        _)))
  (return 0))

(fn OnRepEnableMOTD
  (if (Variables|Default|GetEnableMOTD)
    (CallFunction|SetMOTD)))

(fn OnRepDiscordURL)

(fn OnRepDiscordInfo)

(fn OnRepRuleInfos)

(fn OnRepDonateInfo)

(fn OnRepDonateURL)

(fn OnRepImageURL)

(fn OnRepBannerURL)

(fn OnRepX)

(fn OnRepY)