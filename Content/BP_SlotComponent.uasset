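; Mordhau slot component that changes the equipment slot count of the character its Controller possesses.
; A looping one-second timer calls a server event, which multicasts a check for a new living character.
; On a change, it force-drops and destroys fists, resizes the equipment inventory from the clamped Slots value and refreshes the HUD.
; After a short delay it calls the character's OnPostProfileAssigned; EndPlay clears the timer.
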(event Custom|ServerSetPlayerPerk
  (CallFunction|MulticastSetPlayerPerk))

(event Custom|MulticastSetPlayerPerk
  (bind _returnvalue (CallFunction|SetCharacter))
  (if _returnvalue
    (CallFunction|ModifySlots)
    (Utilities|FlowControl|Delay 0.2)
    (Class|MordhauCharacter|OnPostProfileAssigned (Variables|Default|GetCharacter))))

(event EventBeginPlay
  (bind _returnvalue (Utilities|Time|SetTimerbyEvent (delegate Custom|ServerSetPlayerPerk) 1.0 true))
  (Variables|Default|SetNewVar_0 _returnvalue))

(event EventTick
  (params (DeltaSeconds :type Float%20%28single-precision%29)))

(event EventEndPlay
  (params (EndPlayReason :type EEndPlayReason%20Enum :default "Destroyed"))
  (Utilities|Time|ClearandInvalidateTimerbyHandle (Variables|Default|GetNewVar_0))
  (|CallParentFunction EndPlayReason))

(fn SetCharacter
  (bind _controller (Variables|Default|GetController))
  (bind _returnvalue (Class|MordhauPlayerController|GetControlledMordhauCharacter _controller true))
  (Utilities|IsValid _controller
    (:Is%20Valid
      (Utilities|IsValid _returnvalue
        (:Is%20Valid
          (if (Class|AdvancedCharacter|GetIsDead _returnvalue)
            (Variables|Default|SetCharacter 0 :!label _label)
            (elif (== (Variables|Default|GetCharacter) _returnvalue)
              _
              (else
                (bind _asbp_mordhau_character (Utilities|Casting|CastToBP_MordhauCharacter _returnvalue)
                  (:then
                    (Variables|Default|SetCharacter _asbp_mordhau_character)
                    (return true))
                  (:CastFailed
                    (goto _label)))))))
        (:Is%20Not%20Valid
          (goto _label))))
    (:Is%20Not%20Valid
      (goto _label)))
  (return false))

(fn ModifySlots
  (bind _character (Variables|Default|GetCharacter))
  (LocalVariables|SetNewLocalVar_0 (Math|Integer|Clamp(Integer) (- (Variables|Default|GetSlots) 1) 1 8))
  (for _array_element (Variables|/Script/Mordhau.MordhauCharacter|GetEquipment _character)
    (Utilities|IsValid _array_element
      (:Is%20Valid
        (bind _asbp_fists_weapon (Utilities|Casting|CastToBP_FistsWeapon _array_element))
        (bind _returnvalue (Class|MordhauCharacter|DropEquipment _character _asbp_fists_weapon true))
        (Actor|DestroyActor _returnvalue))))
  (LocalVariables|SetTemp (Variables|/Script/Mordhau.MordhauCharacter|GetEquipment _character))
  (Variables|/Script/Mordhau.MordhauCharacter|SetEquipmentInventorySize _character (Math|Conversions|ToByte(Integer) (LocalVariables|GetNewLocalVar_0)))
  (for _index (range 0 (LocalVariables|GetNewLocalVar_0))
    (Utilities|IsValid (Utilities|Array|Get(acopy) (LocalVariables|GetTemp) _index)
      (:Is%20Valid
        (Utilities|Array|SetArrayElem (LocalVariables|GetTemp) _index (Utilities|Array|Get(acopy) (LocalVariables|GetTemp) _index) true))
      (:Is%20Not%20Valid
        (Utilities|Array|SetArrayElem (LocalVariables|GetTemp) _index 0 true))))
  (Variables|/Script/Mordhau.MordhauCharacter|SetEquipment _character (LocalVariables|GetTemp))
  (bind _asbp_mordhau_hud (Utilities|Casting|CastToBP_MordhauHUD (HUD|GetHUD (Variables|Default|GetController))))
  (Default|ShowEquipment _asbp_mordhau_hud))

(fn OnRepSlots)