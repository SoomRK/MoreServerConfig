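; Mordhau component that applies flag-driven gameplay modifiers to its Controller's character.
; A looping timer detects each new living character, then applies perks, Dutch fists, random gear or resized inventory slots; FistsOnly is an empty stub.
; Perks are toggled by reassigning a modified profile through the customization replication actor, and random gear draws from the singleton's equipment array.
; With Healing on, the character's killer regains health and stamina.
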(event Custom|ServerSpawnGear
  (CallFunction|RandomGearSpawn))

(event Custom|OnCharacterDied
  (params (Character :type Advanced%20Character%20Object%20Reference))
  (Development|PrintString "OnCharacterDied_HealingComponent")
  (bind _returnvalue (Class|AdvancedCharacter|GetLastNetDamageSource Character))
  (bind _asmordhau_character (Utilities|Casting|CastToMordhauCharacter _returnvalue))
  (Class|AdvancedCharacter|OffsetHealth _asmordhau_character 100 true)
  (Class|MordhauCharacter|OffsetStamina _asmordhau_character 100 true))

(event Custom|ServerCheckCharacter
  (bind _returnvalue (CallFunction|SetCharacter))
  (if _returnvalue
    (Utilities|FlowControl|Delay 0.2)
    (Utilities|FlowControl|Sequence
      (:then_0
        (if (Variables|Default|GetHealing)
          (EventDispatchers|BindEventtoOnCharacterDied (Variables|Default|GetCharacter) (EventDispatchers|CreateEvent :!event Custom|OnCharacterDied))))
      (:then_1
        (if (Variables|Default|GetFistsOnly)
          _))
      (:then_2
        (if (Variables|Default|GetPeasantOnly)
          (CallFunction|AddPerktoCharacter 3)))
      (:then_3
        (if (Variables|Default|GetDwarfOnly)
          (CallFunction|AddPerktoCharacter 11)))
      (:then_4
        (if (Variables|Default|GetDutch)
          (CallFunction|GiveDutchFists)))
      (:then_5
        (if (Variables|Default|GetRandomWeapons)
          (CallFunction|ServerSpawnGear)))
      (:then_6
        (if (not (== (Variables|Default|GetSlots) -1))
          (CallFunction|ModifySlots))))))

(event EventBeginPlay
  (Development|PrintString "BeginPlay_MasterComponent_NEW")
  (Utilities|FlowControl|Delay 0.35)
  (CallFunction|SetEquips)
  (bind _returnvalue (Utilities|Time|SetTimerbyEvent (delegate Custom|ServerCheckCharacter) 1.0 true))
  (Variables|Default|SetNewVar_0 _returnvalue))

(event EventEndPlay
  (params (EndPlayReason :type EEndPlayReason%20Enum :default "Destroyed"))
  (Utilities|Time|ClearandInvalidateTimerbyHandle (Variables|Default|GetNewVar_0))
  (|CallParentFunction EndPlayReason))

(fn AddPerktoCharacter
  (params (Perk :type Byte))
  (bind _character (Variables|Default|GetCharacter))
  (bind _returnvalue (Class|MordhauCharacter|GetCustomizationReplicationActor _character))
  (Utilities|IsValid _returnvalue
    (:Is%20Valid
      (if (Ability|HasAuthority _returnvalue)
        (if (Class|MordhauCharacter|HasPerk _character Perk)
          _
          (else
            (bind _returnvalue_2 (Game|ConstructObjectfromClass "/Script/Mordhau.CharacterProfileBPWrapper" self))
            (bind _output_get (Variables|/Script/Mordhau.CharacterProfileBPWrapper|SetProfile _returnvalue_2 (Variables|/Script/Mordhau.CustomizationReplicationActor|GetLastAssignedProfile _returnvalue)))
            (Class|CharacterProfileBPWrapper|TogglePerk _returnvalue_2 Perk)
            (Class|CustomizationReplicationActor|AssignDatafromProfile _returnvalue _output_get)
            (return)))))
    (:Is%20Not%20Valid
      _))
  (return))

(fn SetCharacter
  (bind _controller (Variables|Default|GetController))
  (bind _returnvalue (Class|MordhauPlayerController|GetControlledMordhauCharacter _controller true))
  (Utilities|IsValid _controller
    (:Is%20Valid
      (Utilities|IsValid _returnvalue
        (:Is%20Valid
          (if (Class|AdvancedCharacter|GetIsDead _returnvalue)
            (Variables|Default|SetCharacter 0 :!label _label)
            (elif (== (Variables|Default|GetCharacter) _returnvalue)
              _
              (else
                (Variables|Default|SetCharacter _returnvalue)
                (return true)))))
        (:Is%20Not%20Valid
          (goto _label))))
    (:Is%20Not%20Valid
      (goto _label)))
  (return false))

(fn OnRepPerk)

(fn GiveDutchFists
  (bind _character (Variables|Default|GetCharacter))
  (bind _equipment (Variables|/Script/Mordhau.MordhauCharacter|GetEquipment _character))
  (bind _output (Utilities|Array|Get(acopy) _equipment 2))
  (Utilities|IsValid _output
    (:Is%20Valid
      (bind _returnvalue (Class|MordhauCharacter|DropEquipment _character _output true))
      (Actor|DestroyActor _returnvalue))
    (:Is%20Not%20Valid
      _))
  (bind _returnvalue_2 (Game|SpawnActorfromClass "/MoreServerConfig/BP_DutchFists.BP_DutchFists_C" (Math|Conversions|ToTransform(Vector) (Transformation|GetActorLocation _character)) "Undefined" 0 _character))
  (Class|MordhauCharacter|PickUp _character _returnvalue_2 -1))

(fn RandomGearSpawn
  (bind _character (Variables|Default|GetCharacter))
  (bind _equipment (Variables|/Script/Mordhau.MordhauCharacter|GetEquipment _character))
  (Development|PrintString "RandomGearSpawn")
  (for _array_element _equipment
    (Utilities|IsValid _array_element
      (:Is%20Valid
        (Utilities|Casting|CastToBP_FistsWeapon _array_element
          (:CastFailed
            (bind _returnvalue (Class|MordhauCharacter|DropEquipment _character _array_element true))
            (Actor|DestroyActor _returnvalue))))))
  (for _index (range 0 (- (Utilities|Array|Length _equipment) 2))
    (bind _returnvalue_2 (Game|SpawnActorfromClass (.OutItem (Utilities|Array|Random (Variables|Default|GetEquipment))) (Math|Conversions|ToTransform(Vector) (Transformation|GetActorLocation _character)) "Undefined" 0 _character))
    (bind _returnvalue_3 (Class|MordhauEquipment|GetRandomCustomization _returnvalue_2 false))
    (Class|MordhauEquipment|AssignCustomization _returnvalue_2 _returnvalue_3)
    (Class|MordhauCharacter|PickUp _character _returnvalue_2 -1)
    (if (== _index 0)
      (Class|MordhauCharacter|SwitchEquipment _character _returnvalue_2))))

(fn SetEquips
  (bind _output_get (LocalVariables|SetNewLocalVar_0 (Class|MordhauSingleton|GetEquipmentArray (Class|MordhauUtilityLibrary|GetMordhauSingleton))))
  (Utilities|Array|Clear (Variables|Default|GetEquipment))
  (for _array_element _output_get
    (Utilities|Array|Add (Variables|Default|GetEquipment) (Utilities|ResolveSoftReference _array_element)))
  (Variables|Default|SetEquipment (Variables|Default|GetEquipment)))

(fn ModifySlots
  (bind _character (Variables|Default|GetCharacter))
  (LocalVariables|SetNewLocalVar_0 (Math|Integer|Clamp(Integer) (- (Variables|Default|GetSlots) 1) 1 8))
  (for _array_element (Variables|/Script/Mordhau.MordhauCharacter|GetEquipment _character)
    (Utilities|IsValid _array_element
      (:Is%20Valid
        (bind _asbp_fists_weapon (Utilities|Casting|CastToBP_FistsWeapon _array_element))
        (bind _returnvalue (Class|MordhauCharacter|DropEquipment _character _asbp_fists_weapon true))
        (Actor|DestroyActor _returnvalue))))
  (LocalVariables|SetTemp (Variables|/Script/Mordhau.MordhauCharacter|GetEquipment _character))
  (Variables|/Script/Mordhau.MordhauCharacter|SetEquipmentInventorySize _character (Math|Conversions|ToByte(Integer) (LocalVariables|GetNewLocalVar_0)))
  (for _index (range 0 (LocalVariables|GetNewLocalVar_0))
    (Utilities|IsValid (Utilities|Array|Get(acopy) (LocalVariables|GetTemp) _index)
      (:Is%20Valid
        (Utilities|Array|SetArrayElem (LocalVariables|GetTemp) _index (Utilities|Array|Get(acopy) (LocalVariables|GetTemp) _index) true))
      (:Is%20Not%20Valid
        (Utilities|Array|SetArrayElem (LocalVariables|GetTemp) _index 0 true))))
  (Variables|/Script/Mordhau.MordhauCharacter|SetEquipment _character (LocalVariables|GetTemp))
  (bind _asbp_mordhau_character (Utilities|Casting|CastToBP_MordhauCharacter _character))
  (Default|GiveFists _asbp_mordhau_character)
  (bind _asbp_mordhau_hud (Utilities|Casting|CastToBP_MordhauHUD (HUD|GetHUD (Variables|Default|GetController))))
  (Default|ShowEquipment _asbp_mordhau_hud))