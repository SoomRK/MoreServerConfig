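; Surfboard equipment that gives its holder floaty movement and a forced emote pose while held.
; Equipping changes gravity, air control and jump velocity and disables ragdoll falling and fall damage; holstering or dropping restores them from class defaults.
; Tick reassigns the emote net motion whenever the board is in the right hand, the motion differs and the character can emote.
; FireProjectile is an empty event.
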(event EventBeginPlay
  (|CallParentFunction) ; This node is disabled and will not be called.\nDrag off pins to build functionality.
)

(event Collision|EventActorBeginOverlap
  (params (OtherActor :type Actor%20Object%20Reference))
  (|CallParentFunction OtherActor) ; This node is disabled and will not be called.\nDrag off pins to build functionality.
)

(event EventTick
  (params (DeltaSeconds :type Float%20%28single-precision%29))
  (bind _returnvalue (Class|MordhauEquipment|GetParentCharacter))
  (bind _returnvalue_2 (Class|MordhauCharacter|GetCurrentNetMotion _returnvalue))
  (bind (_id _motiontype _motionparam0 _motionparam1 _motionparam2 _motiondynamicparam) (Utilities|Struct|BreakNetMotion _returnvalue_2))
  (|CallParentFunction DeltaSeconds)
  (Utilities|IsValid _returnvalue
    (:Is%20Valid
      (if (== (Variables|/Script/Mordhau.MordhauCharacter|GetRightHandEquipment _returnvalue) self)
        (if (not (and (== _motiontype 10) (== _motionparam0 31)))
          (if (Class|MordhauCharacter|CanEmote _returnvalue)
            (Class|MordhauCharacter|AssignNetMotionSimple _returnvalue 10 31)))))
    (:Is%20Not%20Valid
      (Development|PrintString "Player is Not Valid [SurfBoard]" true true "(R=1.000000,G=0.000000,B=0.197368,A=1.000000)" 5.0))))

(event EventFireProjectile
  (params (Origin :type Vector%20%28by%20ref%29 :default "0, 0, 0") (Orientation :type Rotator%20%28by%20ref%29 :default "0, 0, 0") (OwningController :type Controller%20Object%20Reference) (ExpectedDelay :type Float%20%28single-precision%29)))

(event EventOnEquipped
  (params (Character :type Mordhau%20Character%20Object%20Reference))
  (bind _charactermovement (Variables|/Script/Engine.Character|GetCharacterMovement Character))
  (|CallParentFunction Character)
  (Variables|/Script/Engine.CharacterMovementComponent|SetGravityScale _charactermovement 0.2)
  (Variables|/Script/Engine.CharacterMovementComponent|SetAirControl _charactermovement 0.25)
  (Variables|/Script/Engine.CharacterMovementComponent|SetJumpZVelocity _charactermovement 6e+02)
  (Variables|/Script/Mordhau.AdvancedCharacter|SetbDisableRagdollFalling Character true)
  (Variables|/Script/Mordhau.AdvancedCharacter|SetReceivedFallDamageModifier Character 0.0))

(event EventOnHolsteredorDropped
  (params (Character :type Mordhau%20Character%20Object%20Reference))
  (bind _returnvalue (Utilities|GetClass Character))
  (bind _charactermovement (Variables|/Script/Engine.Character|GetCharacterMovement Character))
  (bind _returnvalue_2 (Utilities|GetClass _charactermovement))
  (bind (_bdisableragdollfalling _ragdollfallingstarttime _receivedfalldamagemodifier) (Utilities|GetClassDefaults _returnvalue))
  (bind (_gravityscale _jumpzvelocity _aircontrol) (Utilities|GetClassDefaults _returnvalue_2))
  (|CallParentFunction Character)
  (Variables|/Script/Engine.CharacterMovementComponent|SetGravityScale _charactermovement _gravityscale)
  (Variables|/Script/Engine.CharacterMovementComponent|SetAirControl _charactermovement _aircontrol)
  (Variables|/Script/Engine.CharacterMovementComponent|SetJumpZVelocity _charactermovement _jumpzvelocity)
  (Variables|/Script/Mordhau.AdvancedCharacter|SetbDisableRagdollFalling Character _bdisableragdollfalling)
  (Variables|/Script/Mordhau.AdvancedCharacter|SetReceivedFallDamageModifier Character _receivedfalldamagemodifier))

(fn ConstructionScript
  (|CallParentFunction))