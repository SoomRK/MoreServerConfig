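; Mordhau component that gives a controller's character Dutch fists each time it controls a new living character.
; A looping one-second timer runs through server and multicast-named events to SetCharacter, which caches the controlled character and reports changes.
; On a change, ResetGear destroys the item in equipment slot 2 and equips a spawned BP_DutchFists.
; Despite the perk-themed event names, AddPerkToCharacter, an authority-only profile edit, is never called here.
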(event Custom|ServerSetPlayerPerk
  (CallFunction|MulticastSetPlayerPerk))

(event Custom|MulticastSetPlayerPerk
  (bind _returnvalue (CallFunction|SetCharacter))
  (if _returnvalue
    (CallFunction|ResetGear)))

(event EventBeginPlay
  (Development|PrintString "BeginPlayDwarfComp")
  (bind _returnvalue (Utilities|Time|SetTimerbyEvent (delegate Custom|ServerSetPlayerPerk) 1.0 true))
  (Variables|Default|SetNewVar_0 _returnvalue))

(event EventEndPlay
  (params (EndPlayReason :type EEndPlayReason%20Enum :default "Destroyed"))
  (Utilities|Time|ClearandInvalidateTimerbyHandle (Variables|Default|GetNewVar_0))
  (|CallParentFunction EndPlayReason))

(fn AddPerktoCharacter
  (params (Perk :type Byte))
  (bind _character (Variables|Default|GetCharacter))
  (bind _returnvalue (Class|MordhauCharacter|GetCustomizationReplicationActor _character))
  (Utilities|IsValid _returnvalue
    (:Is%20Valid
      (if (Ability|HasAuthority _returnvalue)
        (if (Class|MordhauCharacter|HasPerk _character Perk)
          _
          (else
            (bind _returnvalue_2 (Game|ConstructObjectfromClass "/Script/Mordhau.CharacterProfileBPWrapper" self))
            (bind _output_get (Variables|/Script/Mordhau.CharacterProfileBPWrapper|SetProfile _returnvalue_2 (Variables|/Script/Mordhau.CustomizationReplicationActor|GetLastAssignedProfile _returnvalue)))
            (Class|CharacterProfileBPWrapper|TogglePerk _returnvalue_2 Perk)
            (Class|CustomizationReplicationActor|AssignDatafromProfile _returnvalue _output_get)
            (return)))))
    (:Is%20Not%20Valid
      _))
  (return))

(fn SetCharacter
  (bind _controller (Variables|Default|GetController))
  (bind _returnvalue (Class|MordhauPlayerController|GetControlledMordhauCharacter _controller true))
  (Development|PrintString "SetCharacter")
  (Utilities|IsValid _controller
    (:Is%20Valid
      (Utilities|IsValid _returnvalue
        (:Is%20Valid
          (if (Class|AdvancedCharacter|GetIsDead _returnvalue)
            (Variables|Default|SetCharacter 0 :!label _label)
            (elif (== (Variables|Default|GetCharacter) _returnvalue)
              _
              (else
                (Variables|Default|SetCharacter _returnvalue)
                (return true)))))
        (:Is%20Not%20Valid
          (goto _label))))
    (:Is%20Not%20Valid
      (goto _label)))
  (return false))

(fn OnRepPerk)

(fn ResetGear
  (bind _character (Variables|Default|GetCharacter))
  (bind _equipment (Variables|/Script/Mordhau.MordhauCharacter|GetEquipment _character))
  (bind _output (Utilities|Array|Get(acopy) _equipment 2))
  (Utilities|IsValid _output
    (:Is%20Valid
      (bind _returnvalue (Class|MordhauCharacter|DropEquipment _character _output true))
      (Actor|DestroyActor _returnvalue))
    (:Is%20Not%20Valid
      _))
  (bind _returnvalue_2 (Game|SpawnActorfromClass "/MoreServerConfig/BP_DutchFists.BP_DutchFists_C" (Math|Conversions|ToTransform(Vector) (Transformation|GetActorLocation _character)) "Undefined" 0 _character))
  (Class|MordhauCharacter|PickUp _character _returnvalue_2 -1))