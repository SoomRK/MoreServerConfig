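; BP_DanceParty is a dance party actor that groups child-actor dancers, a chicken and a goat with a Scott Joplin music cue.
; BeginPlay collects the child actor components into an array, with two dancers listed twice.
; DestroyAll starts a music fade-out and delayed stop, then immediately enables replication on each component and child actor, destroys both, and destroys itself.
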(event Custom|DestroyAll
  (bind _scott_joplin_cue (Variables|Default|GetScott_Joplin_Cue))
  (Audio|Components|Audio|FadeOut _scott_joplin_cue 2.0 0.0 "Linear" :!class /Script/Engine.AudioComponent)
  (Audio|Components|Audio|StopDelayed _scott_joplin_cue 2.0)
  (for _array_element (Variables|Default|GetArray)
    (Class|ActorComponent|SetIsReplicated _array_element true)
    (Networking|SetReplicates (Variables|/Script/Engine.ChildActorComponent|GetChildActor _array_element) true)
    (Actor|DestroyActor (Variables|/Script/Engine.ChildActorComponent|GetChildActor _array_element))
    (Components|DestroyComponent _array_element))
  (Actor|DestroyActor))

(event EventBeginPlay
  (Variables|Default|SetArray (Utilities|Array|MakeArray (Variables|Default|GetChicken) (Variables|Default|GetBP_Dancer) (Variables|Default|GetBP_Dancer5) (Variables|Default|GetBP_Dancer2) (Variables|Default|GetBP_Dancer3) (Variables|Default|GetBP_Dancer4) (Variables|Default|GetBP_Dancer1) (Variables|Default|GetGoat) (Variables|Default|GetBP_Dancer_3) (Variables|Default|GetBP_Dancer_4))))

(fn ConstructionScript)