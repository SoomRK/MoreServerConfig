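; BP_Dancer is a profile-driven dancing character that plays a montage chosen by the gender in its assigned appearance profile.
; After short BeginPlay delays it assigns the profile, starts the dance and sets a looping timer, apparently to replay it.
; Tick turns the mesh by a fixed step each frame, independent of delta time.
; GiveFists is empty, and an older looping PlayAnimation branch is left unconnected.
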(event Custom|CustomEvent_0
  (if (Variables|Default|GetIs%20Female)
    (Class|AdvancedCharacter|PlayAnim "/MoreServerConfig/DancyBoi_Montage_SC_2.DancyBoi_Montage_SC_2" 1.0 false)
    (else
      (Class|AdvancedCharacter|PlayAnim "/MoreServerConfig/DancyBoi_Montage_SC.DancyBoi_Montage_SC" 1.0 false))))

(event EventBeginPlay
  (bind _new_profile (Variables|Default|GetNew%20Profile))
  (Utilities|FlowControl|Delay 0.2)
  (Class|MordhauCharacter|AssignProfile _new_profile)
  (Variables|Default|SetIs%20Female (.bIsFemale (Utilities|Struct|BreakAppearanceCustomization (.AppearanceCustomization (Utilities|Struct|BreakCharacterProfile _new_profile)))))
  (Utilities|FlowControl|Delay 0.5)
  (CallFunction|CustomEvent0)
  (Utilities|Time|SetTimerbyEvent (EventDispatchers|CreateEvent :!event Custom|CustomEvent_0) 0.85 true))

(event EventTick
  (params (DeltaSeconds :type Float%20%28single-precision%29))
  (bind _mesh (Variables|Character|GetMesh))
  (|CallParentFunction DeltaSeconds)
  (Transformation|SetRelativeRotation _mesh (Math|Rotator|Delta(Rotator) (Variables|/Script/Engine.SceneComponent|GetRelativeRotation _mesh) "0,1.000000, 0") false false))

(event EventOnPostProfileAssigned
  (|CallParentFunction))

(fn ConstructionScript
  (|CallParentFunction))

(fn GiveFists)