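; Actor component for Mordhau that shows the local player a message-of-the-day screen with rules, Discord and donation info.
; Tick retries until it finds the local player controller, then waits until it is off the main menu map.
; It starts background and banner downloads from URLs, then builds the widget after a fixed delay, not on download completion.
; Once the widget reports closed, Tick removes it and destroys the component.
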(event Custom|DownloadImages
  (Utilities|FlowControl|Sequence
    (:then_0
      (bind _texture (|DownloadImage (Variables|Default|GetImgURL))
        (:OnSuccess
          (Development|PrintString "Component_DownloadBackground_Success" true true "(R=1.000000,G=0.185487,B=0.000000,A=1.000000)" 5.0)
          (Variables|Default|SetTexture _texture))
        (:OnFail
          (Development|PrintString "Component_DownloadBackground_Fail" true true "(R=1.000000,G=0.185487,B=0.000000,A=1.000000)" 5.0))))
    (:then_1
      (bind _texture_2 (|DownloadImage (Variables|Default|GetBannerURL))
        (:OnSuccess
          (Development|PrintString "Component_DownloadBanner_Success" true true "(R=1.000000,G=0.185487,B=0.000000,A=1.000000)" 5.0)
          (Variables|Default|SetBannerTexture _texture_2))
        (:OnFail
          (Development|PrintString "Component_DownloadBanner_Fail" true true "(R=1.000000,G=0.185487,B=0.000000,A=1.000000)" 5.0))))))

(event Custom|AddMOTDWidget
  (bind _controller (Variables|Default|GetController))
  (CallFunction|DownloadImages)
  (Utilities|IsValid _controller
    (:Is%20Valid
      (Utilities|FlowControl|Delay 1.5)
      (bind _returnvalue (Game|ConstructObjectfromClass "/MoreServerConfig/BP_MOTD_Custom2.BP_MOTD_Custom2_C" _controller (Variables|Default|GetDiscordInfo) (Variables|Default|GetRuleInfos) (Variables|Default|GetDiscordURL) (Variables|Default|GetDonateURL) (Variables|Default|GetDonateInfo) (Variables|Default|GetTexture) (Variables|Default|GetImgURL) (Variables|Default|GetBannerTexture) (Variables|Default|GetX) (Variables|Default|GetY)))
      (UserInterface|Viewport|AddtoViewport _returnvalue 101)
      (Widget|SetVisibility _returnvalue "Collapsed")
      (bind _output_get (Variables|Default|SetMOTDWidget _returnvalue))
      (Default|Show _output_get))))

(event Custom|CreateWidget
  (Utilities|FlowControl|DoOnce false :!label _label
    (:Completed
      (bind _output_get (CallFunction|SetController))
      (Utilities|IsValid _output_get
        (:Is%20Valid
          (bind _returnvalue (Game|ConstructObjectfromClass "/DamnedDepend/ZombiesMode/BP_AlertWidget.BP_AlertWidget_C" _output_get))
          (UserInterface|Viewport|AddtoViewport _returnvalue 999)
          (Variables|Default|SetNewVar_0 _returnvalue))
        (:Is%20Not%20Valid
          (Utilities|FlowControl|Delay 0.2)
          (goto _label Reset))))))

(event EventTick
  (params (DeltaSeconds :type Float%20%28single-precision%29))
  (bind _motdwidget (Variables|Default|GetMOTDWidget))
  (Utilities|FlowControl|Sequence
    (:then_0
      (Utilities|FlowControl|DoOnce false :!label _label
        (:Completed
          (bind _output_get (CallFunction|SetController))
          (Utilities|IsValid _output_get
            (:Is%20Valid
              (bind _output_get_2 (Variables|Default|SetController _output_get))
              (Utilities|FlowControl|DoOnce false :!label _label_2
                (:Completed
                  (if (not (Variables|/Game/Mordhau/Blueprints/BP_MordhauPlayerController.BP_MordhauPlayerController_C|GetIsOnMainMenuMap _output_get_2))
                    (CallFunction|AddMOTDWidget)
                    (else
                      (Utilities|FlowControl|Delay 0.2)
                      (Utilities|FlowControl|Sequence
                        (:then_0
                          (goto _label_2 Reset))
                        (:then_1
                          (goto _label_2))))))))
            (:Is%20Not%20Valid
              (goto _label Reset))))))
    (:then_1
      (Utilities|IsValid _motdwidget
        (:Is%20Valid
          (if (Variables|/MoreServerConfig/BP_MOTD_Custom2.BP_MOTD_Custom2_C|GetWasClosed _motdwidget)
            (Widget|RemovefromParent _motdwidget)
            (Components|DestroyComponent)))
        (:Is%20Not%20Valid
          (Development|PrintString "Component_MOTDWidget_NotValid" true true "(R=1.000000,G=0.185487,B=0.000000,A=1.000000)" 5.0))))))

(event EventEndPlay
  (params (EndPlayReason :type EEndPlayReason%20Enum :default "Destroyed"))
  (|CallParentFunction EndPlayReason))

(fn SetController
  (bind _returnvalue (Game|GetPlayerController 0))
  (if (Pawn|IsLocalPlayerController _returnvalue)
    (bind _asbp_mordhau_player_controller (Utilities|Casting|CastToBP_MordhauPlayerController _returnvalue)
      (:then
        (bind _output_get (LocalVariables|SetTemp _asbp_mordhau_player_controller))
        (return _output_get))
      (:CastFailed
        _)))
  (return 0))

(fn SetCharacter
  (bind _controller (Variables|Default|GetController))
  (bind _returnvalue (Class|MordhauPlayerController|GetControlledMordhauCharacter _controller true))
  (Development|PrintString "SetCharacter")
  (Utilities|IsValid _controller
    (:Is%20Valid
      (Utilities|IsValid _returnvalue
        (:Is%20Valid
          (if (Class|AdvancedCharacter|GetIsDead _returnvalue)
            (Variables|Default|SetCharacter 0 :!label _label)
            (elif (== (Variables|Default|GetCharacter) _returnvalue)
              _
              (else
                (Variables|Default|SetCharacter _returnvalue)
                (return true)))))
        (:Is%20Not%20Valid
          (goto _label))))
    (:Is%20Not%20Valid
      (goto _label)))
  (return false))