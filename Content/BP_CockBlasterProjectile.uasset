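; BP_CockBlasterProjectile is a chicken projectile that gibs the characters it kills.
; On a kill, it randomly queues partial dismemberment of head and limb bones, with force derived from projectile-to-victim distance and direction.
; On hit, it spawns cosmetic blood and feathers, then shortly sets the chicken AnimBP's Dead value.
; After a further delay, it repeats the effects, hides the mesh and destroys itself.
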(event EventOnUsedtoKillOther
  (params (Character :type Advanced%20Character%20Object%20Reference) (Type :type EMordhauDamageType%20Enum :default "Generic") (SubType :type Byte :default 0) (Bone :type Name :default "None") (Point :type Vector :default "0, 0, 0") (Source :type Actor%20Object%20Reference))
  (|CallParentFunction Character Type SubType Bone Point Source)
  (bind _asmordhau_character (Utilities|Casting|CastToMordhauCharacter Character))
  (Variables|Default|SetKilledChar _asmordhau_character)
  (for _array_element (Utilities|Array|MakeArray "head" "RightArm" "RightForearm" "RightHand" "LeftArm" "LeftForearm" "LeftHand" "RightUpLeg" "RightLeg" "RightFoot" "LeftUpLeg" "LeftLeg" "LeftFoot")
    (if (Math|Random|RandomBoolwithWeight 0.3)
      (Class|MordhauCharacter|QueueDismember (Variables|Default|GetKilledChar) _array_element true false (Math|Vector|ClampVectorSize (/ (* (Math|Vector|Normalize (- (Transformation|GetWorldLocation (Variables|Default|GetCollisionComp)) (Transformation|GetWorldLocation (Variables|/Script/Engine.Character|GetCapsuleComponent (Variables|Default|GetKilledChar))))) (- 6e+02 (Math|Vector|VectorLength (- (Transformation|GetWorldLocation (Variables|Default|GetCollisionComp)) (Transformation|GetWorldLocation (Variables|/Script/Engine.Character|GetCapsuleComponent (Variables|Default|GetKilledChar))))))) 6e+01) 1.0 8e+02) self))))

(event EventOnProjectileHit
  (params (HitLocation :type Vector :default "0, 0, 0") (HitNormal :type Vector :default "0, 0, 0") (BounceForce :type Float%20%28single-precision%29) (Surface :type Byte :default 0) (bHasHitWorld :type Boolean) (bHasStopped :type Boolean))
  (|CallParentFunction HitLocation HitNormal BounceForce Surface bHasHitWorld bHasStopped)
  (Utilities|FlowControl|Sequence
    (:then_0
      (Networking|CanExecuteCosmeticEvents :!label _label
        (:True
          (Effects|SpawnEmitteratLocation "/Game/Mordhau/Particles/Blood/P_BloodSplash.P_BloodSplash" HitLocation)
          (Effects|SpawnEmitteratLocation "/Game/Mordhau/Assets/Animals/FarmAnimalsPack/Chicken/Effects/P_ChickenFeathers.P_ChickenFeathers" HitLocation))))
    (:then_1
      (Utilities|FlowControl|Delay 0.3)
      (bind _asab_chicken (Utilities|Casting|CastToAB_Chicken (Components|SkeletalMesh|GetAnimInstance (Variables|Default|GetSkeletalMeshComponent)))
        (:then
          (Variables|/MoreServerConfig/AB_Chicken.AB_Chicken_C|SetDead _asab_chicken 1.0)
          (Utilities|FlowControl|Delay 3.0)
          (Utilities|FlowControl|Sequence
            (:then_0
              (goto _label))
            (:then_1
              (Development|SetHiddeninGame (Variables|Default|GetSkeletalMeshComponent) true true)
              (Actor|DestroyActor))))
        (:CastFailed
          (Development|PrintString "cast failed AB_Chicken"))))))

(event EventFire
  (|CallParentFunction))

(event EventOnProjectileFired
  (|CallParentFunction))

(event EventBeginPlay
  (|CallParentFunction))

(fn ConstructionScript
  (|CallParentFunction))