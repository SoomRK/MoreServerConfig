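; Mordhau component that effectively disables AFK removal for the local player by setting a very high MaxAFKTime on their controller.
; One second after BeginPlay, SetController casts player controller 0 to BP_MordhauPlayerController if it is local; a valid result is stored and triggers SetAFKTime.
; SetAFKTime writes the limit with debug logging, retrying every five seconds while the stored controller is invalid.
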(event Custom|SetAFKTime
  (bind _controller (Variables|Default|GetController))
  (Utilities|IsValid _controller :!label _label
    (:Is%20Valid
      (Variables|/Script/Mordhau.MordhauPlayerController|SetMaxAFKTime _controller 99999.0)
      (Development|PrintString "Event: Set AFK Time Complete" true true "(R=1.000000,G=0.000000,B=0.000000,A=1.000000)" 4.0)
      (Class|MordhauUtilityLibrary|PrinttoConsoleandLog "Event: Set AFK Time Complete" false))
    (:Is%20Not%20Valid
      (Utilities|FlowControl|Delay 5.0)
      (goto _label))))

(event EventBeginPlay
  (Utilities|FlowControl|Delay 1.0)
  (bind _output_get (CallFunction|SetController))
  (Utilities|IsValid _output_get
    (:Is%20Valid
      (Variables|Default|SetController _output_get)
      (CallFunction|SetAFKTime)
      (Development|PrintString "Event: Set AFK Time" true true "(R=1.000000,G=0.000000,B=0.000000,A=1.000000)" 4.0)
      (Class|MordhauUtilityLibrary|PrinttoConsoleandLog "Event: Set AFK Time " false))))

(event EventTick
  (params (DeltaSeconds :type Float%20%28single-precision%29)))

(event EventEndPlay
  (params (EndPlayReason :type EEndPlayReason%20Enum :default "Destroyed"))
  (|CallParentFunction EndPlayReason))

(fn SetController
  (bind _returnvalue (Game|GetPlayerController 0))
  (if (Pawn|IsLocalPlayerController _returnvalue)
    (bind _asbp_mordhau_player_controller (Utilities|Casting|CastToBP_MordhauPlayerController _returnvalue)
      (:then
        (bind _output_get (LocalVariables|SetTemp _asbp_mordhau_player_controller))
        (return _output_get))
      (:CastFailed
        _)))
  (return 0))